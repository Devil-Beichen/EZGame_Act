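; Character Blueprint that handles hit reactions to incoming damage through an ActionType state of Normal, KnockOff or KnockDown.
; AnyDamage reads the action from a DamageType_Act damage type, sets the state and plays a matching Frank hit montage.
; Normal hits keep an airborne reaction on knocked-off characters and have no effect on knocked-down ones.
; KnockDown starts a timer to GetUp, which restores Normal, while KnockOff clears that timer.
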(event EventBeginPlay)

(event Collision|EventActorBeginOverlap
  (params (OtherActor :type Actor%20Object%20Reference)))

(event EventTick
  (params (DeltaSeconds :type Float%20%28single-precision%29)))

(fn ConstructionScript)

(fn GetUp
  (Variables|Default|SetActionType "NewEnumerator0"))

(fn KnockDown
  (Variables|Default|SetActionType "NewEnumerator2")
  (Utilities|Time|SetTimerbyFunctionName 0 "GetUp" 2.0))

(fn KnockOff
  (Variables|Default|SetActionType "NewEnumerator1")
  (Utilities|Time|ClearTimerbyFunctionName 0 "GetUp"))

(event Game|Damage|EventAnyDamage
  (params (Damage :type Float%20%28single-precision%29) (DamageType :type Damage%20Type%20Object%20Reference) (InstigatedBy :type Controller%20Object%20Reference) (DamageCauser :type Actor%20Object%20Reference))
  (bind _asdamage_type_act (Utilities|Casting|CastToDamageType_Act DamageType))
  (switch Utilities|FlowControl|Switch|SwitchonEActionType (Variables|/Game/Blueprints/Skill/DamageType_Act.DamageType_Act_C|GetActionType _asdamage_type_act)
    (:NewEnumerator0
      (switch Utilities|FlowControl|Switch|SwitchonEActionType (Variables|Default|GetActionType)
        (:NewEnumerator0
          (Variables|Default|SetActionType "NewEnumerator0")
          (Animation|PlayAnimMontage "/Game/Mannequin/Animations_Act/12_Frank_Hit_high_Montage.12_Frank_Hit_high_Montage" 1.0 "None")
          (CallFunction|GetUp))
        (:NewEnumerator1
          (Variables|Default|SetActionType "NewEnumerator1")
          (Animation|PlayAnimMontage "/Game/Mannequin/Animations_Act/15_Frank_Hit_Air_Montage.15_Frank_Hit_Air_Montage" 1.0 "None")
          (CallFunction|KnockOff :!label _label))))
    (:NewEnumerator1
      (Variables|Default|SetActionType "NewEnumerator1")
      (Animation|PlayAnimMontage "/Game/Mannequin/Animations_Act/15_Frank_Hit_Air_Montage.15_Frank_Hit_Air_Montage" 1.0 "None")
      (goto _label))
    (:NewEnumerator2
      (Variables|Default|SetActionType "NewEnumerator2")
      (Animation|PlayAnimMontage "/Game/Mannequin/Animations_Act/16_Frank_Hit_Bound_Montage.16_Frank_Hit_Bound_Montage" 1.0 "None")
      (CallFunction|KnockDown))))