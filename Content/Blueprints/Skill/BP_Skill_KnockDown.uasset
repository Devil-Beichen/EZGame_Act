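; BP_Skill_KnockDown is a skill that deals light damage with a knock-down damage type to pawns just in front of its owner.
; DoDamage runs a stationary box trace ahead of the owner, with debug drawing on, gathers unique hit actors and applies damage to each.
; OnCastImp is empty and nothing in this graph calls DoDamage, so its trigger lies outside the visible logic.
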(event EventBeginPlay)

(event EventTick
  (params (DeltaSeconds :type Float%20%28single-precision%29)))

(event EventOnCastImp)

(fn DoDamage
  (bind _returnvalue (Components|GetOwner))
  (bind _actorrs (LocalVariables|GetActorrs))
  (bind _returnvalue_2 (Transformation|GetActorLocation _returnvalue))
  (bind _returnvalue_3 (Transformation|GetActorForwardVector _returnvalue))
  (bind _returnvalue_4 (* _returnvalue_3 1e+02))
  (bind _returnvalue_5 (+ _returnvalue_2 _returnvalue_4))
  (bind (_outhits _returnvalue_6) (Class|KismetSystemLibrary|BoxTraceMultiforObjects _returnvalue_5 _returnvalue_5 "50.000000,50.000000,50.000000" (Transformation|GetActorRotation _returnvalue) (Utilities|Array|MakeArray "ObjectTypeQuery3") false 0 "ForDuration" true "(R=1.000000,G=0.000000,B=0.000000,A=1.000000)" "(R=0.000000,G=1.000000,B=0.000000,A=1.000000)" 1.0))
  (if _returnvalue_6
    (for _array_element _outhits
      (Utilities|Array|AddUnique (LocalVariables|GetActorrs) (.HitActor (Collision|BreakHitResult _array_element))))
    (if (Utilities|Array|IsValidIndex _actorrs)
      (for _array_element_2 _actorrs
        (Game|Damage|ApplyDamage _array_element_2 5.0 0 (Components|GetOwner) "/Game/Blueprints/Skill/DamageType_Act_KnockDowm.DamageType_Act_KnockDowm_C")))))